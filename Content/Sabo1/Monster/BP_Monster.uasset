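; Monster Blueprint, apparently a boss, that sets a "Monster" collision profile and applies the GE_BossInit gameplay effect on BeginPlay.
; TakeDamage accumulates damage and plays a timeline that eases YellowHealth toward current health as a trailing health value, clearing the accumulated damage as it advances.
; Surviving hits trigger a world camera shake, while a lethal hit briefly slows global time before the timeline plays.
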(event `self.ReceiveBeginPlay`
  (`PrimitiveComponent.SetCollisionProfileName` (`self.CapsuleComponent`) "Monster" true)
  (`AbilitySystemComponent.BP_ApplyGameplayEffectToSelf` :`self` (`self.AbilitySystemComponent`) :`GameplayEffectClass` "/Game/ThirdPerson/GameplayEffect/GE_BossInit.GE_BossInit_C")
  (`KismetSystemLibrary.Delay` 0.2)
  (set `self.YellowHealth` (`self.GetMaxHealth`)))

(event `self.ReceiveTick`
  (params (DeltaSeconds :type "Float (single-precision)")))

(event `self.TakeDamage`
  (params (Damage :type "Float (double-precision)") (Attacker :type "Actor Object Reference"))
  (bind _returnvalue (+ Damage (`self.Damaged`)))
  (`parent.TakeDamage` Damage Attacker)
  (if (> (`self.GetHealth`) 0.0)
    (set `self.Damaged` _returnvalue)
    (`GameplayStatics.PlayWorldCameraShake` "/Game/ThirdPerson/Collision/MonsterCollisionCameraShake.MonsterCollisionCameraShake_C" (0.0 0.0 0.0) 0.0 100000.0)
    (bind (_direction `_새_트랙_0`) (`Timeline|타임라인` :!via `PlayFromStart` :!label _label)
      (:`Update`
        (set `self.YellowHealth` (`KismetMathLibrary.Lerp` (`self.YellowHealth`) (`self.GetHealth`) `_새_트랙_0`))
        (if (> `_새_트랙_0` 0.0)
          (set `self.Damaged` 0.0))))
    (else
      (set `self.Damaged` _returnvalue)
      (`GameplayStatics.SetGlobalTimeDilation` 0.1)
      (`KismetSystemLibrary.Delay` 0.1)
      (`GameplayStatics.SetGlobalTimeDilation` 1.0)
      (goto _label :!via `PlayFromStart`))))

(fn `UserConstructionScript`
  (`parent.UserConstructionScript`))